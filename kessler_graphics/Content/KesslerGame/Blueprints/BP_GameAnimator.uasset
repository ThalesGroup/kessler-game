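; Renders an externally simulated Kessler asteroid game from text messages received over UDP, sending "graphics_ready" every tick.
; Start messages size the map, position the camera, spawn colored ships and add team tiles, while Score messages fill the scoreboard.
; Frame messages are parsed into asteroid, bullet and ship arrays.
; A 60 Hz timer matches asteroid and bullet mesh component counts to that data and updates all transforms.
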(event `self.UDP.OnReceivedBytes`
  (params (Bytes :type "Array of Byte (by ref)") (IPAddress :type String))
  (bind _returnvalue (`KismetStringLibrary.ParseIntoArray` (`CUBlueprintLibrary.Conv_BytesToString` Bytes) "::"))
  (for (_array_element _array_index) _returnvalue
    (if (== (mod (+ _array_index 1) 2) 0)
      (switch `string` (`|GetArrayItem` _returnvalue (- _array_index 1))
        (:`start`
          (`self.InitializeGame` _array_element)
          (`self.StartGameTimer`))
        (:`frame`
          (`self.UpdateSpriteData` _array_element))
        (:`score`
          (`self.UpdateScoreboard` _array_element))))))

(event `self.ReceiveBeginPlay`)

(event `StartGameTimer`
  (`KismetSystemLibrary.K2_ClearAndInvalidateTimerHandle` (`self.GameTimer`))
  (bind _returnvalue (`KismetSystemLibrary.K2_SetTimerDelegate` (delegate `UpdateGame`) (/ 1.0 60.0) true))
  (set `self.GameTimer` _returnvalue))

(event `UpdateGame`
  (`self.ResizeArrays`)
  (`self.UpdateAsteroids`)
  (`self.UpdateBullets`)
  (for (_array_element _array_index) (`self.ShipsData`)
    (bind _output (`|GetArrayItem` (`self.ShipActors`) _array_index))
    (`/Engine/EditorBlueprintResources/StandardMacros.IsValid` _output
      (:`Is Valid`
        (`/Game/KesslerGame/Blueprints/BP_Ship.UpdateSizeLocRot` _output _array_element)))))

(event `self.ReceiveTick`
  (params (DeltaSeconds :type "Float (single-precision)"))
  (`UDPComponent.EmitBytes` (`self.UDP`) (`CUBlueprintLibrary.Conv_StringToBytes` "graphics_ready")))

(fn `InitializeGame`
  (params (DataString :type String))
  (bind _returnvalue (`GameplayStatics.GetPlayerController` 0))
  (bind _gamescale (`self.GameScale`))
  (bind _camerapoint (`self.CameraPoint`))
  (`|ExecutionSequence`
    (:`then_0`
      (for _array_element (`SceneComponent.GetChildrenComponents` (`self.AsteroidsRoot`) false)
        (`ActorComponent.K2_DestroyComponent` _array_element)))
    (:`then_1`
      (for _array_element_2 (`SceneComponent.GetChildrenComponents` (`self.BulletsRoot`) false)
        (`ActorComponent.K2_DestroyComponent` _array_element_2)))
    (:`then_2`
      (bind _outactors (`GameplayStatics.GetAllActorsOfClass` "/Game/KesslerGame/Blueprints/BP_Ship.BP_Ship_C"))
      (for _array_element_3 _outactors
        (`self.K2_DestroyActor` _array_element_3))
      (`KismetArrayLibrary.Array_Clear` (`self.ShipActors`)))
    (:`then_3`
      (for _array_element_4 (`KismetStringLibrary.ParseIntoArray` DataString ";")
        (bind (_lefts _rights) (`KismetStringLibrary.Split` _array_element_4 ":"))
        (switch `string` _lefts
          (:`map`
            (bind (_lefts_2 _rights_2) (`KismetStringLibrary.Split` _rights ","))
            (bind _returnvalue_2 (* (`KismetStringLibrary.Conv_StringToDouble` _lefts_2) _gamescale))
            (bind _returnvalue_3 (* (`KismetStringLibrary.Conv_StringToDouble` _rights_2) _gamescale))
            (`self.ResizeMap` _returnvalue_2 _returnvalue_3)
            (`|ExecutionSequence`
              (:`then_0`
                (`self.K2_SetActorLocation` (`Controller.K2_GetPawn` _returnvalue) (`SceneComponent.K2_GetComponentLocation` _camerapoint) false true)
                (`Controller.SetControlRotation` _returnvalue (`SceneComponent.RelativeRotation` _camerapoint)))
              (:`then_1`
                (bind _asbp_camera_orb (cast `/Game/KesslerGame/Blueprints/BP_CameraOrb` (`Controller.K2_GetPawn` (`GameplayStatics.GetPlayerController` 0))))
                (bind _camera (`/Game/KesslerGame/Blueprints/BP_CameraOrb.Camera` _asbp_camera_orb))
                (`SceneComponent.K2_SetRelativeRotation` :`self` _camera)
                (`CameraComponent.SetProjectionMode` _camera "Perspective")
                (`CameraComponent.SetOrthoWidth` _camera (+ (`KismetMathLibrary.FMax` _returnvalue_2 (* _returnvalue_3 2.0)) 100.0)))))
          (:`ships`
            (for _index (range (`KismetStringLibrary.Conv_StringToInt` _rights))
              (bind _returnvalue_4 (`|SpawnActorFromClass` "/Game/KesslerGame/Blueprints/BP_Ship.BP_Ship_C" (`KismetMathLibrary.MakeTransform` (0.0 0.0 0.0)) "Undefined" "OverrideRootScale" null null))
              (`KismetArrayLibrary.Array_Add` (`self.ShipActors`) _returnvalue_4)
              (`MaterialInstanceDynamic.SetVectorParameterValue` (`/Game/KesslerGame/Blueprints/BP_Ship.ShipAccentMaterial` _returnvalue_4) "AccentColor" (`|GetArrayItem` (`self.ShipColors`) _index))))
          (:`teams`
            (for _ (range (`KismetStringLibrary.Conv_StringToInt` _rights))
              (`/Game/KesslerGame/UI/UI_Scoreboard.Add Team Tile` (`/Game/KesslerGame/Blueprints/BP_KesslerController.Scoreboard` (cast `/Game/KesslerGame/Blueprints/BP_KesslerController` (`GameplayStatics.GetPlayerController` 0) :!pure true))))))))))

(fn `ResizeArrays`
  (bind _returnvalue (`KismetArrayLibrary.Array_Length` (`self.AsteroidsData`)))
  (bind _returnvalue_2 (`KismetArrayLibrary.Array_Length` (`self.BulletsData`)))
  (bind _returnvalue_3 (`KismetArrayLibrary.Array_Length` (`SceneComponent.GetChildrenComponents` (`self.BulletsRoot`) false)))
  (bind _returnvalue_4 (`KismetArrayLibrary.Array_Length` (`SceneComponent.GetChildrenComponents` (`self.AsteroidsRoot`) false)))
  (bind _output (`|GetArrayItem` (`SceneComponent.GetChildrenComponents` (`self.BulletsRoot`) false)))
  (bind _output_2 (`|GetArrayItem` (`SceneComponent.GetChildrenComponents` (`self.AsteroidsRoot`) false)))
  (while (!= _returnvalue_4 _returnvalue)
    (if (> _returnvalue_4 _returnvalue)
      (`/Engine/EditorBlueprintResources/StandardMacros.IsValid` _output_2
        (:`Is Valid`
          (bind _asstatic_mesh_component (cast `StaticMeshComponent` _output_2))
          (`ActorComponent.K2_DestroyComponent` _asstatic_mesh_component)))
      (else
        (bind _returnvalue_5 (`AddComponent|NODE_AddStaticMeshComponent-0` :`bManualAttachment` true))
        (`StaticMeshComponent.SetStaticMesh` _returnvalue_5 "/Game/KesslerGame/Meshes/SM_Asteroid.SM_Asteroid")
        (`PrimitiveComponent.SetMaterial` _returnvalue_5 0 "/Game/KesslerGame/Materials/M_Asteroid.M_Asteroid")
        (`SceneComponent.K2_AttachToComponent` _returnvalue_5 (`self.AsteroidsRoot`) "None" "KeepRelative" "KeepRelative" "KeepRelative" true))))
  (while (!= _returnvalue_3 _returnvalue_2)
    (if (> _returnvalue_3 _returnvalue_2)
      (`/Engine/EditorBlueprintResources/StandardMacros.IsValid` _output
        (:`Is Valid`
          (bind _asstatic_mesh_component_2 (cast `StaticMeshComponent` _output))
          (`ActorComponent.K2_DestroyComponent` _asstatic_mesh_component_2)))
      (else
        (bind _returnvalue_6 (`AddComponent|NODE_AddStaticMeshComponent-1` :`bManualAttachment` true))
        (`StaticMeshComponent.SetStaticMesh` _returnvalue_6 "/Engine/BasicShapes/Sphere.Sphere")
        (`PrimitiveComponent.SetMaterial` _returnvalue_6 0 "/Game/KesslerGame/Materials/M_Bullet.M_Bullet")
        (`SceneComponent.K2_AttachToComponent` _returnvalue_6 (`self.BulletsRoot`) "None" "KeepRelative" "KeepRelative" "KeepRelative" true))))
  (return))

(fn `ResizeMap`
  (params (Dim1 :type "Float (double-precision)") (Dim2 :type "Float (double-precision)"))
  (bind _returnvalue (* Dim1 0.5))
  (bind _returnvalue_2 (* Dim2 0.5))
  (bind _returnvalue_3 (* Dim2 0.01))
  (bind _returnvalue_4 (* Dim1 0.01))
  (bind _gamewall1 (`self.GameWall1`))
  (bind _gamewall3 (`self.GameWall3`))
  (bind _gamewall2 (`self.GameWall2`))
  (bind _gamewall4 (`self.GameWall4`))
  (bind _returnvalue_5 (`KismetMathLibrary.FMax` _returnvalue_4 _returnvalue_3))
  (bind _returnvalue_6 (* _returnvalue_5 0.05))
  (`|ExecutionSequence`
    (:`then_0`
      (`SceneComponent.K2_SetRelativeTransform` (`self.GameMap`) (`KismetMathLibrary.MakeTransform` (`KismetMathLibrary.MakeVector` _returnvalue _returnvalue_2 -100.0) (struct) (`KismetMathLibrary.MakeVector` _returnvalue_4 _returnvalue_3 _returnvalue_5)) false true))
    (:`then_1`
      (`SceneComponent.SetRelativeScale3D` _gamewall1 (`KismetMathLibrary.MakeVector` _returnvalue_6 _returnvalue_3 0.1))
      (`SceneComponent.K2_SetRelativeLocation` _gamewall1 (`KismetMathLibrary.MakeVector` Dim1 _returnvalue_2) false true))
    (:`then_2`
      (`SceneComponent.SetRelativeScale3D` _gamewall3 (`KismetMathLibrary.MakeVector` _returnvalue_6 _returnvalue_3 0.1))
      (`SceneComponent.K2_SetRelativeLocation` _gamewall3 (`KismetMathLibrary.MakeVector` 0.0 _returnvalue_2) false true))
    (:`then_3`
      (`SceneComponent.SetRelativeScale3D` _gamewall2 (`KismetMathLibrary.MakeVector` _returnvalue_4 _returnvalue_6 0.1))
      (`SceneComponent.K2_SetRelativeLocation` _gamewall2 (`KismetMathLibrary.MakeVector` _returnvalue Dim2) false true))
    (:`then_4`
      (`SceneComponent.SetRelativeScale3D` _gamewall4 (`KismetMathLibrary.MakeVector` _returnvalue_4 _returnvalue_6 0.1))
      (`SceneComponent.K2_SetRelativeLocation` _gamewall4 (`KismetMathLibrary.MakeVector` _returnvalue 0.0) false true))))

(fn `UpdateAsteroids`
  (for (_array_element _array_index) (`SceneComponent.GetChildrenComponents` (`self.AsteroidsRoot`) false)
    (if (not (`ActorComponent.IsBeingDestroyed` _array_element))
      (bind _asstatic_mesh_component (cast `StaticMeshComponent` _array_element))
      (bind (_x _y _angle _radius) (break `/Game/KesslerGame/Blueprints/BP_KesslerObjStruct` (`|GetArrayItem` (`self.AsteroidsData`) _array_index)))
      (bind _returnvalue (`SceneComponent.GetRelativeTransform` _asstatic_mesh_component))
      (bind _returnvalue_2 (* _radius 0.02))
      (`SceneComponent.K2_SetRelativeTransform` _asstatic_mesh_component (`KismetMathLibrary.MakeTransform` (`KismetMathLibrary.MakeVector` _x _y (.z (.location _returnvalue))) (`KismetMathLibrary.MakeRotator` (.roll (.rotation _returnvalue)) (.pitch (.rotation _returnvalue)) _angle) (`KismetMathLibrary.MakeVector` _returnvalue_2 _returnvalue_2 _returnvalue_2)) false true))))

(fn `UpdateBullets`
  (bind _returnvalue (* 0.04 (`self.GameScale`)))
  (for (_array_element _array_index) (`SceneComponent.GetChildrenComponents` (`self.BulletsRoot`) false)
    (if (not (`ActorComponent.IsBeingDestroyed` _array_element))
      (bind _asstatic_mesh_component (cast `StaticMeshComponent` _array_element))
      (bind (_x _y _angle _radius) (break `/Game/KesslerGame/Blueprints/BP_KesslerObjStruct` (`|GetArrayItem` (`self.BulletsData`) _array_index)))
      (bind _returnvalue_2 (`SceneComponent.GetRelativeTransform` _asstatic_mesh_component))
      (`SceneComponent.K2_SetRelativeTransform` _asstatic_mesh_component (`KismetMathLibrary.MakeTransform` (`KismetMathLibrary.MakeVector` _x _y (.z (.location _returnvalue_2))) (`KismetMathLibrary.MakeRotator` (.roll (.rotation _returnvalue_2)) (.pitch (.rotation _returnvalue_2)) _angle) (`KismetMathLibrary.MakeVector` (* _radius 0.02) _returnvalue _returnvalue)) false true)
      (bind _returnvalue_3 (* _radius -1.0))
      (`SceneComponent.K2_AddRelativeLocation` _asstatic_mesh_component (`KismetMathLibrary.MakeVector` (* (`KismetMathLibrary.DegCos` _angle) _returnvalue_3) (* (`KismetMathLibrary.DegSin` _angle) _returnvalue_3)) false false))))

(fn `UpdateScoreboard`
  (params (DataString :type String))
  (locals (Scoreboard :type "/Game/KesslerGame/UI/UI_Scoreboard Object Reference") (Scores :type "Array of /Game/KesslerGame/Blueprints/BP_ScoreStruct Structure"))
  (bind _returnvalue (`KismetStringLibrary.ParseIntoArray` DataString ";"))
  (`|ExecutionSequence`
    (:`then_0`
      (set `local.Scoreboard` (`/Game/KesslerGame/Blueprints/BP_KesslerController.Scoreboard` (cast `/Game/KesslerGame/Blueprints/BP_KesslerController` (`GameplayStatics.GetPlayerController` 0) :!pure true))))
    (:`then_1`
      (for (_array_element _array_index) _returnvalue
        (if (== (mod (+ _array_index 1) 2) 0)
          (switch `string` (`|GetArrayItem` _returnvalue (- _array_index 1))
            (:`time`
              (`TextBlock.SetText` (`/Game/KesslerGame/UI/UI_Scoreboard.sim_time` (`local.Scoreboard`)) (`KismetTextLibrary.Conv_DoubleToText` (`KismetStringLibrary.Conv_StringToDouble` _array_element) "HalfToEven" false true 2 4 2 2)))
            (:`team`
              (bind _returnvalue_2 (`KismetStringLibrary.ParseIntoArray` _array_element ","))
              (`KismetArrayLibrary.Array_Add` (`local.Scores`) (make `/Game/KesslerGame/Blueprints/BP_ScoreStruct` (`KismetStringLibrary.Conv_StringToInt` (`|GetArrayItem` _returnvalue_2)) (`KismetStringLibrary.Conv_StringToInt` (`|GetArrayItem` _returnvalue_2 1)) (`KismetStringLibrary.Conv_StringToInt` (`|GetArrayItem` _returnvalue_2 2)) (`KismetStringLibrary.Conv_StringToInt` (`|GetArrayItem` _returnvalue_2 3)) (`KismetStringLibrary.Conv_StringToDouble` (`|GetArrayItem` _returnvalue_2 4)))))))))
    (:`then_2`
      (for (_array_element_2 _array_index_2) (`PanelWidget.GetAllChildren` (`/Game/KesslerGame/UI/UI_Scoreboard.team_box` (`local.Scoreboard`)))
        (bind _asui_team_tile (cast `/Game/KesslerGame/UI/UI_TeamTile` _array_element_2))
        (`|ExecutionSequence`
          (:`then_0`
            (bind (_output_team _output_asteroids_hit _output_lives_remaining _output_bullets_remaining _output_accuracy) (break `/Game/KesslerGame/Blueprints/BP_ScoreStruct` (`|GetArrayItem` (`local.Scores`) _array_index_2)))
            (`TextBlock.SetText` (`/Game/KesslerGame/UI/UI_TeamTile.team_label` _asui_team_tile) (`KismetTextLibrary.Conv_StringToText` (`KismetStringLibrary.Concat_StrStr` "Team " (`KismetStringLibrary.Conv_IntToString` _output_team) " (" (`|GetArrayItem` (`|MakeArray` "Red" "Blue" "Green" "Yellow") _array_index_2) ")"))))
          (:`then_1`
            (`TextBlock.SetText` (`/Game/KesslerGame/UI/UI_TeamTile.asteroids_hit_val` _asui_team_tile) (`KismetTextLibrary.Conv_IntToText` _output_asteroids_hit)))
          (:`then_2`
            (`TextBlock.SetText` (`/Game/KesslerGame/UI/UI_TeamTile.lives_val` _asui_team_tile) (`KismetTextLibrary.Conv_IntToText` _output_lives_remaining)))
          (:`then_3`
            (`TextBlock.SetText` (`/Game/KesslerGame/UI/UI_TeamTile.bullets_remaining_val` _asui_team_tile) (`KismetTextLibrary.Conv_IntToText` _output_bullets_remaining)))
          (:`then_4`
            (`TextBlock.SetText` (`/Game/KesslerGame/UI/UI_TeamTile.accuracy_val` _asui_team_tile) (`KismetTextLibrary.Conv_DoubleToText` _output_accuracy "HalfToEven" false true 1 2 1 1))))))))

(fn `UpdateSpriteData`
  (params (DataString :type String))
  (`KismetArrayLibrary.Array_Clear` (`self.ShipsData`))
  (`KismetArrayLibrary.Array_Clear` (`self.BulletsData`))
  (`KismetArrayLibrary.Array_Clear` (`self.AsteroidsData`))
  (for _array_element (`KismetStringLibrary.ParseIntoArray` DataString ";")
    (switch `string` (`KismetStringLibrary.GetSubstring` _array_element)
      (:`a`
        (bind _returnvalue (`KismetStringLibrary.ParseIntoArray` (`KismetStringLibrary.RightChop` (`KismetStringLibrary.LeftChop` _array_element 1) 2) ","))
        (bind _bp_kesslerobjstruct (make `/Game/KesslerGame/Blueprints/BP_KesslerObjStruct` (* (`KismetStringLibrary.Conv_StringToDouble` (`|GetArrayItem` _returnvalue)) (`self.GameScale`)) (* (`KismetStringLibrary.Conv_StringToDouble` (`|GetArrayItem` _returnvalue 1)) (`self.GameScale`)) (`KismetStringLibrary.Conv_StringToDouble` (`|GetArrayItem` _returnvalue 2)) (* (`KismetStringLibrary.Conv_StringToDouble` (`|GetArrayItem` _returnvalue 3)) (`self.GameScale`)) (`KismetStringLibrary.EqualEqual_StrStr` (`|GetArrayItem` _returnvalue 4) "1") (`KismetStringLibrary.Conv_StringToDouble` (`|GetArrayItem` _returnvalue 5))))
        (`KismetArrayLibrary.Array_Add` (`self.AsteroidsData`) _bp_kesslerobjstruct))
      (:`s`
        (`KismetArrayLibrary.Array_Add` (`self.ShipsData`) _bp_kesslerobjstruct))
      (:`b`
        (`KismetArrayLibrary.Array_Add` (`self.BulletsData`) _bp_kesslerobjstruct)))))

(fn `UserConstructionScript`
  (set `self.ShipColors` (`|MakeArray` (make `LinearColor` 0.33 0.04 0.04) (make `LinearColor` 0.04 0.04 0.4) (make `LinearColor` 0.04 0.2 0.04) (make `LinearColor` 0.3 0.2 0.04))))