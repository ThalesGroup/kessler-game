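; BP_Ship is the visual actor for a ship in KesslerGame, driven by externally supplied state rather than its own logic.
; The construction script creates dynamic materials for the shield sphere and ship mesh.
; UpdateSizeLocRot teleports the actor to the struct's X/Y and yaw, scales it from radius, and feeds respawn time to the shield material.
; When the struct reports the ship is not alive, the actor destroys itself.
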(fn `UpdateSizeLocRot`
  (params (InStruct :type "/Game/KesslerGame/Blueprints/BP_KesslerObjStruct Structure"))
  (bind (_x _y _angle _radius _alive _respawntime) (break `/Game/KesslerGame/Blueprints/BP_KesslerObjStruct` InStruct))
  (bind _returnvalue (`self.GetTransform`))
  (bind _returnvalue_2 (* _radius 0.02))
  (if _alive
    (`self.K2_SetActorTransform` (`KismetMathLibrary.MakeTransform` (`KismetMathLibrary.MakeVector` _x _y (.z (.location _returnvalue))) (`KismetMathLibrary.MakeRotator` (.roll (.rotation _returnvalue)) (.pitch (.rotation _returnvalue)) _angle) (`KismetMathLibrary.MakeVector` _returnvalue_2 _returnvalue_2 _returnvalue_2)) false true)
    (`MaterialInstanceDynamic.SetScalarParameterValue` (`self.ShieldMaterial`) "RespawnTime" _respawntime)
    (else
      (`self.K2_DestroyActor`))))

(fn `UserConstructionScript`
  (`|ExecutionSequence`
    (:`then_0`
      (bind _returnvalue (`KismetMaterialLibrary.CreateDynamicMaterialInstance` "/Game/KesslerGame/Materials/M_ShieldMaterial.M_ShieldMaterial"))
      (bind _output_get (set `self.ShieldMaterial` _returnvalue))
      (`PrimitiveComponent.SetMaterial` (`self.Sphere`) 0 _output_get))
    (:`then_1`
      (bind _returnvalue_2 (`KismetMaterialLibrary.CreateDynamicMaterialInstance` "/Game/KesslerGame/Materials/M_Ship_lambert3SG.M_Ship_lambert3SG"))
      (bind _output_get_2 (set `self.ShipAccentMaterial` _returnvalue_2))
      (`PrimitiveComponent.SetMaterial` (`self.ShipMesh`) 0 _output_get_2))))