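; BP_CameraOrb is a free-flying camera pawn moved by player axis input.
; Forward/backward, left/right and up/down axes feed the FloatingPawnMovement component along the Camera's forward, right and up vectors, so movement is relative to the camera's orientation.
; Pitch and Yaw axis events are empty, with their controller rotation nodes left disconnected, so this graph applies no look rotation.
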(event `InputAxis|ForwardBackward`
  (params (AxisValue :type "Float (single-precision)"))
  (`PawnMovementComponent.AddInputVector` (`self.FloatingPawnMovement`) (* AxisValue (`SceneComponent.GetForwardVector` (`self.Camera`))) false))

(event `InputAxis|LeftRight`
  (params (AxisValue :type "Float (single-precision)"))
  (`PawnMovementComponent.AddInputVector` (`self.FloatingPawnMovement`) (* AxisValue (`SceneComponent.GetRightVector` (`self.Camera`))) false))

(event `InputAxis|UpDown`
  (params (AxisValue :type "Float (single-precision)"))
  (`PawnMovementComponent.AddInputVector` (`self.FloatingPawnMovement`) (* AxisValue (`SceneComponent.GetUpVector` (`self.Camera`))) false))

(event `InputAxis|Pitch`
  (params (AxisValue :type "Float (single-precision)")))

(event `InputAxis|Yaw`
  (params (AxisValue :type "Float (single-precision)")))

(event `self.ReceiveTick`
  (params (DeltaSeconds :type "Float (single-precision)")))

(fn `UserConstructionScript`)